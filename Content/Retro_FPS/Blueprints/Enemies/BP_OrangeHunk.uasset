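; BP_OrangeHunk is a Paper2D flipbook melee enemy for the retro FPS that chases and hurts the player.
; Pawn sensing starts an AI move toward the player and clears CanSeePlayer, the flag that gates yaw-only facing on Tick.
; Capsule hits against the tagged player call EnemyHit with fixed damage.
; Any damage triggers a one-time death: movement deactivates, death flipbooks play, and the actor is destroyed.
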(event OnSeePawn(PawnSensing)
  (params (Pawn :type Pawn%20Object%20Reference))
  ;[1 1 1] Enemy Move Towards Player
  (bind _asbp_fpsplayer (Utilities|Casting|CastToBP_FPSPlayer Pawn))
  (Variables|Default|SetCanSeePlayer false)
  (AI|AIMoveTo self "0, 0, 0" _asbp_fpsplayer 3.0 false))

(event OnComponentHit(CapsuleComponent)
  (params (HitComponent :type Primitive%20Component%20Object%20Reference) (OtherActor :type Actor%20Object%20Reference) (OtherComp :type Primitive%20Component%20Object%20Reference) (NormalImpulse :type Vector :default "0, 0, 0") (Hit :type Hit%20Result%20Structure%20%28by%20ref%29))
  ;[1 1 1] Deal Damage
  (if (Actor|ActorHasTag OtherActor "Player")
    (bind _asbp_fpsplayer (Utilities|Casting|CastToBP_FPSPlayer OtherActor))
    (Default|EnemyHit _asbp_fpsplayer 0 1e+01)))

(event EventTick
  (params (DeltaSeconds :type Float%20%28single-precision%29))
  ;[1 1 1] Face Player
  (if (Variables|Default|GetCanSeePlayer)
    (Transformation|SetActorRotation (Math|Rotator|MakeRotator 0.0 0.0 (.yaw (Math|Rotator|FindLookatRotation (Transformation|GetActorLocation) (Transformation|GetActorLocation (Game|GetPlayerCharacter 0))))))))

(event Game|Damage|EventAnyDamage
  (params (Damage :type Float%20%28single-precision%29) (DamageType :type Damage%20Type%20Object%20Reference) (InstigatedBy :type Controller%20Object%20Reference) (DamageCauser :type Actor%20Object%20Reference))
  (bind _paperflipbook (Variables|Default|GetPaperFlipbook))
  ;[1 1 1] Enemy Death
  (Utilities|FlowControl|DoOnce false
    (:Completed
      (Components|Activation|Deactivate (Variables|Character|GetCharacterMovement))
      (Sprite|SetFlipbook _paperflipbook "/Game/Retro_FPS/FlipBooks/FB_EnemyDeath.FB_EnemyDeath")
      (Utilities|FlowControl|Delay (Class|PaperFlipbookComponent|GetFlipbookLength _paperflipbook))
      (Sprite|SetFlipbook (Variables|Default|GetPaperFlipbook) "/Game/Retro_FPS/FlipBooks/FB_DeadIdle.FB_DeadIdle")
      (Utilities|FlowControl|Delay 0.5)
      (Actor|DestroyActor))))

(fn ConstructionScript)