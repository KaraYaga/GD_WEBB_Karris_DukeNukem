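; Base Blueprint for the player's retro FPS weapons, drawn as a flipbook that a scene capture component shows exclusively.
; WeaponBob plays a sequence while moving and otherwise stops it, interpolating the flipbook back to its starting position.
; FireWeapon line-traces forward from the LineTrace component and applies damage to the hit actor, with debug drawing enabled.
; ShootWeapon and StopShooting are empty events, and InitializeWeapon unhides the flipbook.
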(event Custom|WeaponBob
  (params (isMoving :type Boolean) (deltaTime :type Float%20%28double-precision%29))
  (bind _weapon_bob (Variables|Default|GetWeapon%20Bob))
  (bind _weapon_flipbook (Variables|Default|GetWeapon_FlipBook))
  (bind _sequenceplayer (Variables|/Script/ActorSequence.ActorSequenceComponent|GetSequencePlayer _weapon_bob))
  ;[1 1 1] Weapon Bobbing With Player Movement
  (if isMoving
    (Sequencer|Player|Play _sequenceplayer :!class /Script/MovieScene.MovieSceneSequencePlayer)
    (else
      (Sequencer|Player|Stop _sequenceplayer :!class /Script/MovieScene.MovieSceneSequencePlayer)
      (Transformation|SetRelativeLocation _weapon_flipbook (Math|Interpolation|VInterpTo (Variables|/Script/Engine.SceneComponent|GetRelativeLocation _weapon_flipbook) (Variables|Default|GetWeapon%20Position) deltaTime 0.0) false false))))

(event Custom|ShootWeapon)

(event Custom|StopShooting)

(event EventBeginPlay
  ;[1 1 1] Show Weapon / Get Location
  (Rendering|SceneCapture|ShowOnlyComponent (Variables|Default|GetSceneCaptureComponent2D) (Variables|Default|GetWeapon_FlipBook))
  (Variables|Default|SetWeapon%20Position (Variables|/Script/Engine.SceneComponent|GetRelativeLocation (Variables|Default|GetWeapon_FlipBook))))

(event EventInitializeWeapon
  (bind _weapon_flipbook (Variables|Default|GetWeapon_FlipBook))
  (Sprite|SetFlipbook _weapon_flipbook)
  (Development|SetHiddeninGame _weapon_flipbook false false))

(fn ConstructionScript)

(fn FireWeapon
  (bind _linetrace (Variables|Default|GetLineTrace))
  (bind _returnvalue (Transformation|GetWorldLocation _linetrace))
  ;[1 1 1] LIne Trace Fire
  (bind (_outhit _returnvalue_2) (Collision|LineTraceForObjects _returnvalue (+ _returnvalue (* (Math|Vector|GetForwardVector (Transformation|GetWorldRotation (Variables|Default|GetLineTrace))) (Variables|Default|GetLineTraceDistance*))) (Utilities|Array|MakeArray "ObjectTypeQuery1" "ObjectTypeQuery2" "ObjectTypeQuery3") false (Utilities|Array|MakeArray self (Game|GetPlayerCharacter 0)) "ForDuration"))
  (if _returnvalue_2
    (Game|Damage|ApplyDamage (.HitActor (Collision|BreakHitResult _outhit)) (Variables|Default|GetWeapon%20Damage) 0 0)))