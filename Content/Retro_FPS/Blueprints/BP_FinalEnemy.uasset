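; BP_FinalEnemy is a flipbook-sprite bug enemy for the retro FPS that chases the player and can be killed.
; PawnSensing starts AIMoveTo toward a seen BP_FPSPlayer and clears CanSeePlayer, the flag that gates yaw-only player facing on Tick.
; AnyDamage subtracts Health; at exactly zero, it deactivates movement once, plays death and dead flipbooks, then destroys the actor after a delay.
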(event OnSeePawn(PawnSensing)
  (params (Pawn :type Pawn%20Object%20Reference))
  ;[1 1 1] Enemy Move Towards Player
  (bind _asbp_fpsplayer (Utilities|Casting|CastToBP_FPSPlayer Pawn))
  (Variables|Default|SetCanSeePlayer false)
  (AI|AIMoveTo self "0, 0, 0" _asbp_fpsplayer 3.0 false))

(event EventTick
  (params (DeltaSeconds :type Float%20%28single-precision%29))
  ;[1 1 1] Face Player
  (if (Variables|Default|GetCanSeePlayer)
    (Transformation|SetActorRotation (Math|Rotator|MakeRotator 0.0 0.0 (.yaw (Math|Rotator|FindLookatRotation (Transformation|GetActorLocation) (Transformation|GetActorLocation (Game|GetPlayerCharacter 0))))))))

(event Game|Damage|EventAnyDamage
  (params (Damage :type Float%20%28single-precision%29) (DamageType :type Damage%20Type%20Object%20Reference) (InstigatedBy :type Controller%20Object%20Reference) (DamageCauser :type Actor%20Object%20Reference))
  (bind _paperflipbook (Variables|Default|GetPaperFlipbook))
  ;[1 1 1] Enemy Death
  (bind _output_get (Variables|Default|SetHealth (- (Variables|Default|GetHealth) Damage)))
  (if (== _output_get 0.0)
    (Utilities|FlowControl|DoOnce false
      (:Completed
        (Components|Activation|Deactivate (Variables|Character|GetCharacterMovement))
        (Sprite|SetFlipbook _paperflipbook "/Game/Retro_FPS/FlipBooks/FB_BugDeath.FB_BugDeath")
        (Utilities|FlowControl|Delay (Class|PaperFlipbookComponent|GetFlipbookLength _paperflipbook))
        (Sprite|SetFlipbook (Variables|Default|GetPaperFlipbook) "/Game/Retro_FPS/FlipBooks/FB_BugDead.FB_BugDead")
        (Utilities|FlowControl|Delay 4.0)
        (Actor|DestroyActor)))))

(fn ConstructionScript)