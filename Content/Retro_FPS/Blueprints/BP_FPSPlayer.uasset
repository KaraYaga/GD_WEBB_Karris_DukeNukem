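; Player character for a retro FPS, handling movement, mouse look, shooting, health and the win/death screens.
; The equipped weapon spawns through a child actor component, initializes via I_PlayerWeapon, then handles firing and velocity-driven bob each tick.
; Damage drains armor before health, updating the stats widget; health exactly at zero shows the death screen and destroys the player.
; Overlapping any TriggerBox shows the win screen.
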(event Custom|Equip%20Weapon
  (params (Weapon :type BP%20Player%20Weapon%20Base%20Class%20Reference))
  (bind _childactor (Variables|/Script/Engine.ChildActorComponent|GetChildActor (Variables|Default|GetWeapon)))
  ;[1 1 1] Weapon
  ;;[1 1 1] Equip Weapon
  (bind _output_get (Variables|Player|SetCurrent%20Weapon Weapon))
  (ChildActorComponent|SetChildActorClass (Variables|Default|GetWeapon) _output_get)
  (if (Utilities|DoesObjectImplementInterface _childactor "/Game/Retro_FPS/Blueprints/Weapons/I_PlayerWeapon.I_PlayerWeapon_C")
    (Class|IPlayerWeapon|InitializeWeapon(Message) _childactor)
    (bind _asbp_player_weapon_base (Utilities|Casting|CastToBP_PlayerWeaponBase _childactor))
    (bind _output_get_2 (Variables|Default|SetCurrentWeapon _asbp_player_weapon_base))
    (Sequencer|Player|Play (Variables|/Script/ActorSequence.ActorSequenceComponent|GetSequencePlayer (Variables|/Game/Retro_FPS/Blueprints/Weapons/BP_PlayerWeaponBase.BP_PlayerWeaponBase_C|GetWeapon%20Draw _output_get_2)) :!class /Script/MovieScene.MovieSceneSequencePlayer)))

(event Custom|EnemyHit
  (params (DamagedActor :type Actor%20Object%20Reference) (Damage :type Float%20%28single-precision%29) (DamageType :type Damage%20Type%20Object%20Reference) (InstigatedBy :type Controller%20Object%20Reference) (DamageCauser :type Actor%20Object%20Reference))
  (bind _returnvalue (Game|GetPlayerController 0))
  ;[1 1 1] Player Controls and Stats
  ;;[1 1 1] Player Health
  (if (> (Variables|Default|GetArmor) 0.0)
    (Variables|Default|SetArmor (- (Variables|Default|GetArmor) Damage))
    (Rendering|Components|TextRender|SetText (Variables|/Game/Retro_FPS/Blueprints/Widgets/WBP_Stats.WBP_Stats_C|GetT_Armor (Variables|Default|GetHealth_Widget)) (Utilities|Text|ToText(Float) (Variables|Default|GetArmor) "HalfToEven"))
    (else
      (Variables|Default|SetHealth (- (Variables|Default|GetHealth) Damage))
      (Rendering|Components|TextRender|SetText (Variables|/Game/Retro_FPS/Blueprints/Widgets/WBP_Stats.WBP_Stats_C|GetT_Health (Variables|Default|GetHealth_Widget)) (Utilities|Text|ToText(Float) (Variables|Default|GetHealth) "HalfToEven"))
      (if (== (Variables|Default|GetHealth) 0.0)
        (bind _returnvalue_2 (UserInterface|CreateWidget "/Game/Retro_FPS/Blueprints/Widgets/WBP_PlayerDeath.WBP_PlayerDeath_C"))
        (UserInterface|Viewport|AddtoViewport _returnvalue_2 0)
        (Variables|/Script/Engine.PlayerController|SetbShowMouseCursor _returnvalue true)
        (Input|SetInputModeGameandUI _returnvalue 0 "DoNotLock" true false)
        (Actor|DestroyActor)))))

(event EventBeginPlay
  ;[1 1 1] Stats HUD
  (Utilities|FlowControl|Sequence
    (:then_0
      ;;[1 1 1] Weapon HUD
      (bind _returnvalue (UserInterface|CreateWidget "/Game/Retro_FPS/Blueprints/Widgets/WBP_HUD.WBP_HUD_C"))
      (UserInterface|Viewport|AddtoViewport _returnvalue 0)
      (CallFunction|EquipWeapon "/Game/Retro_FPS/Blueprints/Weapons/BP_PlayerWeaponBase.BP_PlayerWeaponBase_C"))
    (:then_1
      ;;[1 1 1] Health
      (bind _returnvalue_2 (UserInterface|CreateWidget "/Game/Retro_FPS/Blueprints/Widgets/WBP_Stats.WBP_Stats_C"))
      (bind _output_get (Variables|Default|SetHealth_Widget _returnvalue_2))
      (UserInterface|Viewport|AddtoPlayerScreen _output_get))))

(event EventTick
  (params (DeltaSeconds :type Float%20%28single-precision%29))
  ;[1 1 1] Weapon
  ;;[1 1 1] Weapon Bob On Move
  (bind _asbp_player_weapon_base (Utilities|Casting|CastToBP_PlayerWeaponBase (Variables|/Script/Engine.ChildActorComponent|GetChildActor (Variables|Default|GetWeapon))))
  (Default|WeaponBob _asbp_player_weapon_base (> (Math|Vector|VectorLength (Variables|/Script/Engine.MovementComponent|GetVelocity (Variables|Character|GetCharacterMovement))) 0.0) DeltaSeconds))

(event Collision|EventActorBeginOverlap
  (params (OtherActor :type Actor%20Object%20Reference))
  (bind _returnvalue (Game|GetPlayerController 0))
  ;[1 1 1] Player Win
  (Utilities|Casting|CastToTriggerBox OtherActor)
  (bind _returnvalue_2 (UserInterface|CreateWidget "/Game/Retro_FPS/Blueprints/Widgets/WBP_PlayerWin.WBP_PlayerWin_C"))
  (UserInterface|Viewport|AddtoViewport _returnvalue_2 0)
  (Variables|/Script/Engine.PlayerController|SetbShowMouseCursor _returnvalue true)
  (Input|SetInputModeGameandUI _returnvalue 0 "DoNotLock" true false))

(event Input|ActionEvents|InputActionShoot
  (params (Key :type Key%20Structure :default "None"))
  (bind _currentweapon (Variables|Default|GetCurrentWeapon))
  ;[1 1 1] Weapon
  ;;[1 1 1] Shoot
  (:Pressed
    (Utilities|IsValid _currentweapon
      (:Is%20Valid
        (Default|ShootWeapon _currentweapon)))))

(event Input|AxisEvents|InputAxisMoustLookVertical
  (params (AxisValue :type Float%20%28single-precision%29))
  ;[1 1 1] Player Controls and Stats
  ;;[1 1 1] Mouse Look
  (Pawn|Input|AddControllerPitchInput AxisValue))

(event Input|AxisEvents|InputAxisVerticalMovement
  (params (AxisValue :type Float%20%28single-precision%29))
  ;[1 1 1] Player Controls and Stats
  ;;[1 1 1] Movement
  (Pawn|Input|AddMovementInput (Math|Vector|GetForwardVector (Math|Rotator|MakeRotator 0.0 0.0 (.yaw (Pawn|GetControlRotation :!class /Script/Engine.Pawn)))) AxisValue false))

(event Input|AxisEvents|InputAxisHorizontalMovement
  (params (AxisValue :type Float%20%28single-precision%29))
  ;[1 1 1] Player Controls and Stats
  ;;[1 1 1] Movement
  (Pawn|Input|AddMovementInput (Math|Vector|GetRightVector (Math|Rotator|MakeRotator 0.0 0.0 (.yaw (Pawn|GetControlRotation :!class /Script/Engine.Pawn)))) (* AxisValue -1.0) false))

(event Input|AxisEvents|InputAxisMouseLookHorizontal
  (params (AxisValue :type Float%20%28single-precision%29))
  ;[1 1 1] Player Controls and Stats
  ;;[1 1 1] Mouse Look
  (Pawn|Input|AddControllerYawInput AxisValue))

(fn ConstructionScript)