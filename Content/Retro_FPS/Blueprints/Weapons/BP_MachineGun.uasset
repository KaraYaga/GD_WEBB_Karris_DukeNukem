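; BP_MachineGun is the machine gun weapon Blueprint for the retro FPS, drawn with a Paper2D flipbook.
; InitializeWeapon sets the idle flipbook and makes it visible.
; ShootWeapon passes a DoOnce gate, calls FireWeapon and plays the firing flipbook.
; After a delay matching that flipbook's length, it restores the idle flipbook and calls ResetWeapon to reopen the gate, so fire rate follows animation length.
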(event Custom|ResetWeapon
  (bind _weapon_flipbook (Variables|Default|GetWeapon_FlipBook))
  ;[1 1 1] Fire and reset
  (Utilities|FlowControl|DoOnce false) ; enters at Reset
)

(event EventShootWeapon
  (bind _weapon_flipbook (Variables|Default|GetWeapon_FlipBook))
  ;[1 1 1] Fire and reset
  (Utilities|FlowControl|DoOnce false
    (:Completed
      (CallFunction|FireWeapon)
      (Sprite|SetFlipbook _weapon_flipbook "/Game/Retro_FPS/FlipBooks/FB_MachineGunFire.FB_MachineGunFire")
      (Utilities|FlowControl|Delay (Class|PaperFlipbookComponent|GetFlipbookLength _weapon_flipbook))
      (Sprite|SetFlipbook (Variables|Default|GetWeapon_FlipBook) "/Game/Retro_FPS/FlipBooks/FB_MachineGunIdle.FB_MachineGunIdle")
      (CallFunction|ResetWeapon))))

(event EventInitializeWeapon
  ;[1 1 1] Weapon Hidden on Pickup
  (Sprite|SetFlipbook (Variables|Default|GetWeapon_FlipBook) (Variables|Default|GetIdle%20MG))
  (Development|SetHiddeninGame (Variables|Default|GetWeapon_FlipBook) false false))

(fn ConstructionScript
  (|CallParentFunction))